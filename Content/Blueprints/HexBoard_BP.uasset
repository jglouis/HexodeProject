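; Hex board actor that lays out a hexagonal playfield, tracks tokens and turns mouse input into move orders.
; The construction script rebuilds instanced tiles within Radius using hex-distance checks, and BeginPlay registers every HexToken_BP after a short delay.
; A cursor trace converts the hit location to a hex coordinate, which moves the highlight mesh each Tick and, on click, goes to HexodePlayerController_BP as a move order.
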(event MouseInput|EventActorOnClicked
  ;[1 1 1] Move token on click
  (bind _hex_coordinate (CallFunction|GetCursorHexCoordinate))
  (bind _ashexode_player_controller_bp (Utilities|Casting|CastToHexodePlayerController_BP (Game|GetPlayerController 0)))
  (Default|OnMoveOrderCoordGiven _ashexode_player_controller_bp _hex_coordinate))

(event EventTick
  (params (DeltaSeconds :type Float%20%28single-precision%29))
  ;[1 1 1] Move highlight cursor when moving over a hex
  (bind _hex_coordinate (CallFunction|GetCursorHexCoordinate))
  (Transformation|SetWorldLocation (Variables|Default|GetCursorOverBoardMesh) (+ (Class|HexBoard|GetWorldLocationfromHexCoordinate _hex_coordinate) "0, 0,1.000000") false false))

(event EventBeginPlay
  ;[1 1 1] Add Tokens to the board
  (Utilities|FlowControl|Delay 1.0)
  (bind _outactors (Actor|GetAllActorsOfClass "/Game/Blueprints/HexToken_BP.HexToken_BP_C"))
  (for _array_element _outactors
    (Class|HexBoard|AddToken _array_element)))

(fn ConstructionScript
  (bind _radius (Variables|Default|GetRadius))
  (bind _returnvalue (Math|Conversions|ToInteger(Byte) _radius))
  (bind _returnvalue_2 (- 0 _returnvalue))
  (Components|InstancedStaticMesh|ClearInstances (Variables|Default|GetBoardMesh))
  (for _index (range _returnvalue_2 _returnvalue)
    (LocalVariables|SetCurrentU _index)
    (for _index_2 (range _returnvalue_2 (Math|Conversions|ToInteger(Byte) _radius))
      (LocalVariables|SetCurrentV _index_2)
      (if (> (Math|Conversions|ToInteger(Byte) (Variables|Default|GetRadius)) (Class|HexUtil|Distance (Utilities|Struct|MakeHexCoordinate (LocalVariables|GetCurrentU) (LocalVariables|GetCurrentV))))
        (Class|HexBoard|DisplayTile (Utilities|Struct|MakeHexCoordinate (LocalVariables|GetCurrentU) (LocalVariables|GetCurrentV)))))))

(fn GetCursorHexCoordinate
  (bind _returnvalue (Game|GetPlayerController 0))
  (bind _array (Utilities|Array|MakeArray "ObjectTypeQuery1"))
  (bind _hitresult (Class|PlayerController|GetHitResultUnderCursorforObjects _returnvalue _array true))
  (bind (_bblockinghit _binitialoverlap _time _location _impactpoint _normal _impactnormal _physmat _hitactor) (Collision|BreakHitResult _hitresult))
  (Utilities|IsValid _returnvalue
    (:Is%20Valid
      (bind _ashex_board (Utilities|Casting|CastToHexBoard _hitactor))
      (return (Class|HexBoard|GetHexCoordfromWorldLocation _ashex_board _location)))
    (:Is%20Not%20Valid
      (return (Utilities|Struct|MakeHexCoordinate 0 0)))))

(fn PrintHexCoordinate
  (params (Coord :type Hex%20Coordinate%20Structure))
  (bind (_u _v) (Utilities|Struct|BreakHexCoordinate Coord))
  (Development|PrintString (Utilities|String|Append "(" (Utilities|String|ToString(Integer) _u) "," (Utilities|String|ToString(Integer) _v) ")")))