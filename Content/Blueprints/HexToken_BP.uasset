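; HexToken_BP is a clickable token actor that glides toward a target location and can be selected.
; Each tick it eases position toward the target with a frame-dependent lerp, turning to face it until within a small distance.
; OnSetTargetLocation updates that target.
; Clicking resets every token's Cone material to default, highlights this one, and reports it to HexodePlayerController_BP as the new selection.
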(event `self.ReceiveTick`
  (params (DeltaSeconds :type "Float (single-precision)"))
  (bind _returnvalue (`self.GetTargetMoveLocation`))
  (bind _returnvalue_2 (`self.K2_GetActorLocation`))
  (`|ExecutionSequence`
    (:`then_0`
      ;[1 1 1] Set orientation
      (if (> (`KismetMathLibrary.VSize` (- _returnvalue_2 _returnvalue)) 10.0)
        (`self.SetActorRotation` (`KismetMathLibrary.RLerp` (`KismetMathLibrary.Conv_VectorToRotator` (`KismetMathLibrary.GetDirectionVector` _returnvalue_2 _returnvalue)) (`self.K2_GetActorRotation`) 0.9))))
    (:`then_1`
      ;[1 1 1] Move to target location
      (`self.K2_SetActorLocation` (`KismetMathLibrary.VLerp` (`self.K2_GetActorLocation`) (`self.GetTargetMoveLocation`) 0.1)))))

(event `OnSetTargetLocation`
  (params (NewTargetLocation :type "Vector Structure"))
  (`KismetSystemLibrary.PrintString` "target")
  (`self.SetTargetMoveLocation` NewTargetLocation))

(event `self.ReceiveActorOnClicked`
  ;[1 1 1] Selection logic on click event
  (`|ExecutionSequence`
    (:`then_0`
      ;;[1 1 1] Set all tokens to default material
      (bind _outactors (`GameplayStatics.GetAllActorsOfClass` "HexToken_BP_C"))
      (for _array_element _outactors
        (`PrimitiveComponent.SetMaterial` (`/Game/Blueprints/HexToken_BP.Cone` _array_element) 0 (`self.Default Material`))))
    (:`then_1`
      ;;[1 1 1] Set this token to selected material
      (`PrimitiveComponent.SetMaterial` (`self.Cone`) 0 (`self.Selected Material`)))
    (:`then_2`
      ;;[1 1 1] Changed selected token on player controller
      (bind _ashexode_player_controller_bp (cast `/Game/Blueprints/HexodePlayerController_BP` (`GameplayStatics.GetPlayerController` 0)))
      (`/Game/Blueprints/HexodePlayerController_BP.OnNewSelectedToken` _ashexode_player_controller_bp self))))

(fn `UserConstructionScript`)