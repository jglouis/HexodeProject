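; HexagonalTileCollision is a clickable hex tile actor that stores its U,V grid coordinates and reports clicks to move a token.
; SetHexagonalCoordinates assigns U and V, and BeginPlay enables click events on the first player controller.
; A click forwards the coordinates to HexodeGameMode_BP's OnClickedTile, while hover and click both print them as debug text.
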(event `self.ReceiveBeginPlay`
  ;[1 1 1] Activate click events
  (set `PlayerController.bEnableClickEvents` true (`GameplayStatics.GetPlayerController` 0)))

(event `self.ReceiveActorBeginCursorOver`
  ;[1 1 1] Print coordinates on cursor over
  (`KismetSystemLibrary.PrintString` (`KismetStringLibrary.Concat_StrStr` "(" (`KismetStringLibrary.Conv_IntToString` (`self.U`)) "," (`KismetStringLibrary.Conv_IntToString` (`self.V`)) ")")))

(event `self.ReceiveActorOnClicked`
  (`|ExecutionSequence`
    (:`then_0`
      ;[1 1 1] Move Token on click
      (bind _ashexode_game_mode_bp (cast `/Game/Blueprints/HexodeGameMode_BP` (`GameplayStatics.GetGameMode`)))
      (`/Game/Blueprints/HexodeGameMode_BP.OnClickedTile` _ashexode_game_mode_bp (`self.U`) (`self.V`)))
    (:`then_1`
      ;[1 1 1] Print coordinates on click
      (`KismetSystemLibrary.PrintString` (`KismetStringLibrary.Concat_StrStr` "Clicked on (" (`KismetStringLibrary.Conv_IntToString` (`self.U`)) "," (`KismetStringLibrary.Conv_IntToString` (`self.V`)) ")")))))

(fn `SetHexagonalCoordinates`
  (params (U :type Integer) (V :type Integer))
  (set `self.U` U)
  (set `self.V` V))

(fn `UserConstructionScript`)