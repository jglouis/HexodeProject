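; Game mode for Hexode that resolves simultaneous turns once every player has ended theirs.
; On Tick, with authority, it checks each player state's HasEndedTurn flag and stops at the first unfinished player.
; When all have finished, it applies each player's MoveOrders by setting token coordinates, then calls OnTurnReset on that player state.
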(event `self.ReceiveTick`
  (params (DeltaSeconds :type "Float (single-precision)"))
  (bind _playerarray (`GameState.PlayerArray` (`GameplayStatics.GetGameState`)))
  ;[1 1 1] End of turn is triggered when all players have finished
  (`/Engine/EditorBlueprintResources/ActorMacros.Switch Has Authority`
    (:`Authority`
      (set `self.ToEnd` true)
      (for _array_element _playerarray
        (bind _ashexode_player_state_bp (cast `/Game/Blueprints/HexodePlayerState_BP` _array_element))
        (if (not (`/Game/Blueprints/HexodePlayerState_BP.HasEndedTurn` _ashexode_player_state_bp))
          (set `self.ToEnd` false)
          (break)))
      (if (`self.ToEnd`)
        (`|ExecutionSequence`
          (:`then_0`
            ;;[1 1 1] Finish
            (`KismetSystemLibrary.PrintString` "end turn on game mode"))
          (:`then_1`
            (for _array_element_2 _playerarray
              (bind _ashexode_player_state_bp_2 (cast `/Game/Blueprints/HexodePlayerState_BP` _array_element_2))
              (`|ExecutionSequence`
                (:`then_0`
                  ;[1 1 1] Set new coordinates
                  (for _array_element_3 (`/Game/Blueprints/HexodePlayerState_BP.MoveOrders` _ashexode_player_state_bp_2)
                    (set `HexToken.Coord` (break `MoveOrder` _array_element_3) (`.Token` (break `MoveOrder` _array_element_3)))))
                (:`then_1`
                  ;[1 1 1] Reset player states
                  (`/Game/Blueprints/HexodePlayerState_BP.OnTurnReset` _ashexode_player_state_bp_2))))))))))

(fn `UserConstructionScript`)