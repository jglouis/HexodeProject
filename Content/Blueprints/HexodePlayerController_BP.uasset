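; Player controller for Hexode, a turn-based game with tokens on hex coordinates, that turns player input into move orders and end-turn requests.
; BeginPlay shows the cursor and enables click and mouse-over events.
; Move orders for the selected token and the T-key end turn are forwarded to HexodePlayerState_BP.
; A separate event, meant to run on the server, sets a token's hex coordinate directly.
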(event `self.ReceiveBeginPlay`
  (bind _returnvalue (`GameplayStatics.GetPlayerController` 0))
  ;[1 1 1] Activate cursor
  (set `PlayerController.bShowMouseCursor` true _returnvalue)
  (set `PlayerController.bEnableMouseOverEvents` true _returnvalue)
  ;[1 1 1] Activate click event
  (set `PlayerController.bEnableClickEvents` true _returnvalue))

(event `OnTokenToBeMoved`
  (params (Token :type "/Game/Blueprints/HexToken_BP Object Reference") (Coord :type "HexCoordinate Structure"))
  ;[1 1 1] Event called on the server to set the token target location
  (`HexToken.SetHexCoordinate` Token Coord))

(event `Key|T`
  (params (Key :type "Key Structure" :default "AnyKey"))
  (:`Pressed`
    (`KismetSystemLibrary.PrintString` "end turn")
    (bind _ashexode_player_state_bp (cast `/Game/Blueprints/HexodePlayerState_BP` (`self.PlayerState`)))
    (`/Game/Blueprints/HexodePlayerState_BP.OnPlayerEndTurn` _ashexode_player_state_bp)))

(event `OnMoveOrderCoordGiven`
  (params (Coord :type "HexCoordinate Structure"))
  ;[1 1 1] Event triggered when a new move order is submitted for the selected token
  (`/Engine/EditorBlueprintResources/StandardMacros.IsValid` (`self.Selected Token`)
    (:`Is Valid`
      (bind _ashexode_player_state_bp (cast `/Game/Blueprints/HexodePlayerState_BP` (`self.PlayerState`)))
      (`/Game/Blueprints/HexodePlayerState_BP.OnAddOrder` _ashexode_player_state_bp (`self.Selected Token`) Coord))))

(fn `OnRep_TurnEnded`)

(fn `UserConstructionScript`)