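; HexodePlayerState_BP is a player state that tracks one player's turn in Hexode, holding an end-of-turn flag and queued move orders.
; OnAddOrder appends a token and its target U/V coordinate to MoveOrders.
; OnPlayerEndTurn sets HasEndedTurn and prints each queued order for debugging, without executing the moves.
; OnTurnReset clears the flag and the order list for a new turn.
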(event `OnPlayerEndTurn`
  ;[1 1 1] Event triggered when a player ends its turn
  (`|ExecutionSequence`
    (:`then_0`
      (set `self.HasEndedTurn` true)
      (`KismetSystemLibrary.PrintString` "end turn on player state"))
    (:`then_1`
      (for _array_element (`self.MoveOrders`)
        (`KismetSystemLibrary.PrintString` (`KismetStringLibrary.Concat_StrStr` (`KismetSystemLibrary.GetDisplayName` (break `MoveOrder` _array_element)) " moves to " "(" (`KismetStringLibrary.Conv_IntToString` (break `HexCoordinate` (`.Coord` (break `MoveOrder` _array_element)))) "," (`KismetStringLibrary.Conv_IntToString` (`.V` (break `HexCoordinate` (`.Coord` (break `MoveOrder` _array_element))))) ")"))))))

(event `OnAddOrder`
  (params (Token :type "/Game/Blueprints/HexToken_BP Object Reference") (Coord :type "HexCoordinate Structure"))
  ;[1 1 1] Add an order
  (`KismetArrayLibrary.Array_Add` (`self.MoveOrders`) (make `MoveOrder` Token Coord)))

(event `OnTurnReset`
  ;[1 1 1] Reset player state when turn is ended
  (set `self.HasEndedTurn` false)
  (`KismetArrayLibrary.Array_Clear` (`self.MoveOrders`)))

(fn `UserConstructionScript`)