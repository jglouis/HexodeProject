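; Vector_BP is an actor that draws a vector between Start and End as an arrow segment mesh.
; Its construction script adds a static mesh component, stretches it along X by the distance between the points over the mesh's base length, aims X from Start to End, and centers it at the midpoint.
; Location is set relative while rotation and scale are set in world space.
; The event graph is empty.
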(event EventBeginPlay)

(event EventActorBeginOverlap
  (params (OtherActor :type Actor%20Object%20Reference)))

(event EventTick
  (params (DeltaSeconds :type Float%20%28single-precision%29)))

(fn ConstructionScript
  (bind _returnvalue (AddComponent|AddStaticMeshComponent false))
  (LocalVariables|Setarrow%20segment _returnvalue)
  (Components|StaticMesh|SetStaticMesh (LocalVariables|Getarrow%20segment) "/Game/Models/arrow_segment.arrow_segment")
  (Utilities|FlowControl|Sequence
    (:then_0
      ;[1 1 1] Set scale
      (Transformation|SetWorldScale3D (LocalVariables|Getarrow%20segment) (Math|Vector|MakeVector (/ (Math|Vector|VectorLength (- (Variables|Default|GetEnd) (Variables|Default|GetStart))) 2e+02) 1.0 1.0)))
    (:then_1
      ;[1 1 1] Set rotation
      (Transformation|SetWorldRotation (LocalVariables|Getarrow%20segment) (Math|Rotator|MakeRotfromX (Class|KismetMathLibrary|GetDirectionVector (Variables|Default|GetStart) (Variables|Default|GetEnd))) false false))
    (:then_2
      ;[1 1 1] Recenter
      (Transformation|SetRelativeLocation (LocalVariables|Getarrow%20segment) (+ (/ (- (Variables|Default|GetEnd) (Variables|Default|GetStart)) 2) (Variables|Default|GetStart)) false false))))